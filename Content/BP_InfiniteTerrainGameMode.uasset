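; Game mode for an infinite terrain game that spawns chained tiles and tracks a score of conquered tiles.
; On BeginPlay it populates a pool of nav mesh bounds volumes, then spawns the first two tiles.
; Each spawned BP_Tile receives the shared pool, and its attach location becomes the spawn transform for the next tile.
; NewTileConquered increments the score, which GetScore exposes.
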(event EventBeginPlay
  (Class|InfiniteTerrainGameMode|PopulateVolumeBoundsPool)
  (for _index (range 0 1)
    (CallFunction|SpawnTile)))

(fn ConstructionScript)

(fn SpawnTile
  (bind _returnvalue (Game|SpawnActorfromClass "/Game/Terrain/BP_Tile.BP_Tile_C" (Variables|Default|GetSpawnTransform) "Undefined" 0 0))
  (Class|Tile|SetPool _returnvalue (Variables|Default|GetNavMeshBoundsVolumePool))
  (bind _transform (Default|GetAttachLocation _returnvalue))
  (Variables|Default|SetSpawnTransform _transform))

(fn NewTileConquered
  (Math|Integer|IncrementInt (Variables|Default|GetScore)))

(fn GetScore
  (return (Variables|Default|GetScore)))